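; BP_ShootingHUD is the shooting game's HUD Blueprint, passing the player's health, ammo and magazine values to the on-screen widget.
; Each OnUpdateMy event casts HudWidget to ShootingHudWidget and calls the matching SetHp, SetAmmo or SetMag, doing nothing if the cast fails.
; The graph neither creates the widget nor polls for values, as BeginPlay, Tick and the construction script are empty.
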(event EventBeginPlay)

(event Collision|EventActorBeginOverlap
  (params (OtherActor :type Actor%20Object%20Reference)))

(event EventTick
  (params (DeltaSeconds :type Float%20%28single-precision%29)))

(event EventOnUpdateMyHp
  (params (CurHp :type Float%20%28single-precision%29) (MaxHp :type Float%20%28single-precision%29))
  (bind _asshooting_hud_widget (Utilities|Casting|CastToShootingHudWidget (Variables|Default|GetHudWidget)))
  (Default|SetHp _asshooting_hud_widget CurHp MaxHp))

(event EventOnUpdateMyAmmo
  (params (Ammo :type Integer))
  (bind _asshooting_hud_widget (Utilities|Casting|CastToShootingHudWidget (Variables|Default|GetHudWidget)))
  (Default|SetAmmo _asshooting_hud_widget Ammo))

(event EventOnUpdateMyMag
  (params (Mag :type Integer))
  (bind _asshooting_hud_widget (Utilities|Casting|CastToShootingHudWidget (Variables|Default|GetHudWidget)))
  (Default|SetMag _asshooting_hud_widget Mag))

(fn ConstructionScript)