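; BP_Weapon is a weapon actor for the shooting game that a character can pick up, drop, fire and reload.
; Pickup stores the owner and attaches the physics-disabled mesh to its "weapon" socket; drop reverses this, and only an unowned weapon can be picked up.
; Trigger and reload play montages on the owner.
; Shoot is a separate function that only spawns a small explosion effect and sound at the muzzle, without traces or damage.
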(event EventBeginPlay)

(event Collision|EventActorBeginOverlap
  (params (OtherActor :type Actor%20Object%20Reference)))

(event EventTick
  (params (DeltaSeconds :type Float%20%28single-precision%29)))

(fn ConstructionScript)

(fn EventDrop
  (params (Character :type Character%20Object%20Reference))
  (bind _staticmesh (Variables|Default|GetStaticMesh))
  (Variables|Default|SetOwnChar 0)
  (Physics|SetSimulatePhysics _staticmesh true)
  (Transformation|DetachFromComponent _staticmesh "KeepWorld" "KeepWorld" "KeepWorld" true)
  (return false))

(fn EventPickUp
  (params (Character :type Character%20Object%20Reference))
  (bind _output_get (Variables|Default|SetOwnChar Character))
  (Physics|SetSimulatePhysics (Variables|Default|GetStaticMesh) false)
  (Transformation|AttachComponentToComponent self (Variables|/Script/Engine.Character|GetMesh _output_get) "weapon" "SnapToTarget" "SnapToTarget" "KeepWorld" true))

(fn EventReload
  (Animation|PlayAnimMontage (Variables|Default|GetOwnChar) (Variables|Default|GetReloadMontage) 1.0 "None")
  (return true))

(fn EventShoot
  (bind _staticmesh (Variables|Default|GetStaticMesh))
  (Effects|SpawnEmitteratLocation "/Game/StarterContent/Particles/P_Explosion.P_Explosion" (Transformation|GetSocketLocation _staticmesh "muzzle") (Transformation|GetSocketRotation _staticmesh "None") "0.100000,0.100000,0.100000")
  (Audio|SpawnSoundatLocation "/Game/StarterContent/Audio/Explosion_Cue.Explosion_Cue" (Transformation|GetSocketLocation (Variables|Default|GetStaticMesh) "muzzle") "0, 0, 0" 1.0 1.0 0.0 0 0)
  (return true))

(fn EventTrigger
  (Animation|PlayAnimMontage (Variables|Default|GetOwnChar) (Variables|Default|GetShootMontage) 1.0 "None")
  (return true))

(fn IsCanPickup
  (Utilities|IsValid (Variables|Default|GetOwnChar)
    (:Is%20Valid
      (return false))
    (:Is%20Not%20Valid
      (return true))))