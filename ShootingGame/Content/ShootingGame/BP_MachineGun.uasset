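; BP_MachineGun is a machine gun weapon for the shooting game that gives automatic fire while the trigger is held.
; EventTrigger plays the shoot montage on press and starts a looping timer by function name to replay it at a fixed interval, clearing the timer on release.
; LoopShootMontage plays ShootMontage on the owning character, and the file itself contains no projectile or damage logic.
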(event EventBeginPlay)

(event Collision|EventActorBeginOverlap
  (params (OtherActor :type Actor%20Object%20Reference)))

(event EventTick
  (params (DeltaSeconds :type Float%20%28single-precision%29)))

(fn ConstructionScript
  (|CallParentFunction))

(fn EventTrigger
  (params (bIsPress :type Boolean))
  (if bIsPress
    (CallFunction|LoopShootMontage)
    (Utilities|Time|SetTimerbyFunctionName 0 "LoopShootMontage" 0.2 true)
    (else
      (Utilities|Time|ClearTimerbyFunctionName 0 "LoopShootMontage")))
  (return false))

(fn LoopShootMontage
  (Animation|PlayAnimMontage (Variables|Default|GetOwnChar) (Variables|Default|GetShootMontage) 1.0 "None"))