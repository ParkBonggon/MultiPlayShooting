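; BP_ShootingPlayerState is the shooting game's player state and holds the player's current and maximum HP.
; CurrentHP starts at MaxHP on BeginPlay, and AddDamage subtracts damage from it without clamping.
; A RepNotify on CurrentHP prints the new value and fires the UpdateMyHP dispatcher with current and max HP, so listeners can react to health changes.
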(event EventBeginPlay
  (Variables|Default|SetCurrentHP (Variables|Default|GetMaxHP)))

(fn ConstructionScript)

(fn AddDamage
  (params (Damage :type Float%20%28double-precision%29))
  (Variables|Default|SetCurrentHP (- (Variables|Default|GetCurrentHP) Damage)))

(fn OnRepCurrentHP
  (Development|PrintString (Utilities|String|Append "Current HP" (Utilities|String|ToString(Float) (Variables|Default|GetCurrentHP))))
  (Default|CallDispatcherUpdateMyHP (Variables|Default|GetCurrentHP) (Variables|Default|GetMaxHP)))