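; BP_ShootingGameHud is the shooting game's HUD Blueprint, putting HP and ammo on screen.
; On BeginPlay it creates the HUD widget, then binds to the player state's HP update dispatcher and pushes the current values.
; If the player state cast fails, a short timer retries the binding until it succeeds.
; SetHudHP and SetHudAmmo forward values to the widget.
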(event EventBeginPlay
  (bind _returnvalue (UserInterface|CreateWidget "/Game/ShootingGame/Wedget/ShootingHudWidget.ShootingHudWidget_C"))
  (bind _output_get (Variables|Default|SetHud%20Widget _returnvalue))
  (UserInterface|Viewport|AddtoViewport _output_get 0)
  (CallFunction|BindMyPlayerState))

(fn ConstructionScript)

(fn SetHudHP
  (params (CurHp :type Float%20%28double-precision%29) (MaxHp :type Float%20%28double-precision%29))
  (Default|SetHP (Variables|Default|GetHud%20Widget) CurHp MaxHp))

(fn BindMyPlayerState
  (bind _asbp_shooting_player_state (Utilities|Casting|CastToBP_ShootingPlayerState (Variables|/Script/Engine.Controller|GetPlayerState (Game|GetPlayerController 0)))
    (:then
      (EventDispatchers|BindEventtoDispatcherUpdateMyHP _asbp_shooting_player_state (EventDispatchers|CreateEvent :!event SetHudHP))
      (CallFunction|SetHudHP (Variables|/Game/ShootingGame/GameMode/BP_ShootingPlayerState.BP_ShootingPlayerState_C|GetCurrentHP _asbp_shooting_player_state) (Variables|/Game/ShootingGame/GameMode/BP_ShootingPlayerState.BP_ShootingPlayerState_C|GetMaxHP _asbp_shooting_player_state)))
    (:CastFailed
      (Utilities|Time|SetTimerbyFunctionName 0 "BindMyPlayerState" 0.01))))

(fn SetHudAmmo
  (params (Ammo :type Byte))
  (Default|SetAmmo (Variables|Default|GetHud%20Widget) Ammo))